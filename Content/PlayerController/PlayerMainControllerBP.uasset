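; Player controller Blueprint that turns raw input bindings into queued actions and movement input.
; Attack, Crouch and Jump presses and releases feed separate instances of a polling-queue node, each press tagged with its action type.
; The four directional axis events converge on one SetMovementInput call, which receives summed axis values as X and Y.
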(event `InputAction|Attack`
  (params (Key :type "Key Structure"))
  (:`Pressed`
    (`PlayerInputPollingSystem.AddActionToUserInputPollingQueue` (`self.PlayerInputPollingSystem`) "ATTACK" :!label _label))
  (:`Released`
    (goto _label :!via `Released`)))

(event `InputAction|Crouch`
  (params (Key :type "Key Structure"))
  (:`Pressed`
    (`PlayerInputPollingSystem.AddActionToUserInputPollingQueue` (`self.PlayerInputPollingSystem`) "CROUCH" :!label _label_2))
  (:`Released`
    (goto _label_2 :!via `Released`)))

(event `InputAction|Jump`
  (params (Key :type "Key Structure"))
  (:`Pressed`
    (`PlayerInputPollingSystem.AddActionToUserInputPollingQueue` (`self.PlayerInputPollingSystem`) "JUMP" :!label _label_3))
  (:`Released`
    (goto _label_3 :!via `Released`)))

(event `InputAxis|Move_Left`
  (params (AxisValue :type "Float (single-precision)"))
  (`self.SetMovementInput` (+ AxisValue (stale `InputAxis|Move_Right` AxisValue)) (+ (stale `InputAxis|Move_Forward` AxisValue) (stale `InputAxis|Move_Backward` AxisValue)) :!label _label_4))

(event `InputAxis|Move_Right`
  (params (AxisValue :type "Float (single-precision)"))
  (goto _label_4))

(event `InputAxis|Move_Forward`
  (params (AxisValue :type "Float (single-precision)"))
  (goto _label_4))

(event `InputAxis|Move_Backward`
  (params (AxisValue :type "Float (single-precision)"))
  (goto _label_4))

(fn `UserConstructionScript`)